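; BP_PlayerState is a player state that stores the player's name and runs the round timer.
; On BeginPlay it passes the player name to SendMyNameToServer, which saves it in MyName, and starts a timer using the Time variable.
; When the timer fires, RoundEnd disables input on the owner, shows WBP_ScoreBoard, then quits the game after a delay.
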(event `self.ReceiveBeginPlay`
  (`self.Send My Name to Server` (`KismetTextLibrary.Conv_StringToText` (`self.GetPlayerName`)))
  (bind _returnvalue (`KismetSystemLibrary.K2_SetTimerDelegate` (delegate `Round End`) (`self.Time`)))
  (set `self.Timer` _returnvalue))

(event `Send My Name to Server`
  (params (MyName :type Text))
  (set `self.MyName` MyName))

(event `Round End`
  (`self.DisableInput` (`self.GetOwner`) (`GameplayStatics.GetPlayerController` 0))
  (bind _returnvalue (`|CreateWidget` "/Game/UI/WBP_ScoreBoard.WBP_ScoreBoard_C" (`self.GetPlayerController`)))
  (`UserWidget.AddToViewport` _returnvalue 0)
  (`KismetSystemLibrary.Delay` 20.0)
  (`KismetSystemLibrary.QuitGame` (`self.GetPlayerController`) "Quit"))

(fn `UserConstructionScript`)